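; BP_LevelMap is the level map actor that switches between two tile map layouts when the mask changes.
; On BeginPlay it assigns both tile maps, shows the first with collision and binds to the change-mask delegate.
; Each delegate event toggles visibility and collision so only the tile map matching mask 1 or 2 is active.
; A FirstRun flag suppresses the mask-change sound on the first event.
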(event Custom|OnChangeMaskDelegateFired
  (params (mask :type Integer))
  (if (Variables|Default|GetFirstRun)
    (Audio|PlaySound2D "/Game/Assets/Sound/New__Mask_Change_Sounds_effect__mp3cut_net_.New__Mask_Change_Sounds_effect__mp3cut_net_" 0.5 1.0 0.0 0 0)
    (else
      (Variables|Default|SetFirstRun true)))
  (switch int mask
    (:1
      (Rendering|SetVisibility (Variables|Default|GetStaticTiles1) true true)
      (Rendering|SetVisibility (Variables|Default|GetStaticTiles2) false true)
      (Collision|SetCollisionEnabled (Variables|Default|GetStaticTiles1) "QueryAndPhysics")
      (Collision|SetCollisionEnabled (Variables|Default|GetStaticTiles2) "NoCollision"))
    (:2
      (Rendering|SetVisibility (Variables|Default|GetStaticTiles1) false true)
      (Rendering|SetVisibility (Variables|Default|GetStaticTiles2) true true)
      (Collision|SetCollisionEnabled (Variables|Default|GetStaticTiles1) "NoCollision")
      (Collision|SetCollisionEnabled (Variables|Default|GetStaticTiles2) "QueryAndPhysics"))))

(event EventBeginPlay
  (Variables|Default|SetFirstRun false)
  (Class|PaperTileMapComponent|SetTileMap (Variables|Default|GetStaticTiles1) (Variables|Default|GetTMBase1))
  (Class|PaperTileMapComponent|SetTileMap (Variables|Default|GetStaticTiles2) (Variables|Default|GetTMBase2))
  (Rendering|SetVisibility (Variables|Default|GetStaticTiles1) true true)
  (Rendering|SetVisibility (Variables|Default|GetStaticTiles2) false true)
  (Collision|SetCollisionEnabled (Variables|Default|GetStaticTiles1) "QueryAndPhysics")
  (Collision|SetCollisionEnabled (Variables|Default|GetStaticTiles2) "NoCollision")
  (EventDispatchers|BindEventtoChangeMaskDelegate (delegate Custom|OnChangeMaskDelegateFired)))

(event EventTick
  (params (DeltaSeconds :type Float%20%28single-precision%29)))

(fn ConstructionScript)